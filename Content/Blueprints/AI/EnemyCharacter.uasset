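; EnemyCharacter is an AI enemy that patrols between two route points and ends the game on contact with the player.
; On BeginPlay it calls IrARuta, which moves it to a random navigable point near RutaInicial or RutaFinal.
; Whether the move succeeds or fails, it calls itself with the flag flipped, looping endlessly between the two ends.
; Overlapping a Jugador actor calls that player's GameOver.
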(event Custom|IrARuta
  (params (EsRutaInicial :type Boolean))
  (AI|AIMoveTo self (.RandomLocation (Class|NavigationSystemV1|GetRandomPointinNavigableRadius (Math|Vector|SelectVector (Transformation|GetActorLocation (Variables|Default|GetRutaInicial)) (Transformation|GetActorLocation (Variables|Default|GetRutaFinal)) EsRutaInicial) 5e+01 0 0)) 0 5.0 false
    (:OnSuccess
      _)
    (:OnFail
      _))
  (CallFunction|IrARuta (not EsRutaInicial)))

(event EventBeginPlay
  (CallFunction|IrARuta true))

(event Collision|EventActorBeginOverlap
  (params (OtherActor :type Actor%20Object%20Reference))
  (bind _asjugador (Utilities|Casting|CastToJugador OtherActor))
  (Default|GameOver _asjugador))

(fn ConstructionScript)